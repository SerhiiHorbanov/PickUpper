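; Actor component that lets its owner pick up whatever actor it is facing.
; Each tick it line-traces on Visibility from the owner's location, along the control rotation for pawn owners or actor forward otherwise, out to a pickup distance, and stores the hit actor.
; TryPickUp sends that actor a PickUpMessage with the owner as argument.
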(event EventTick
  (params (DeltaSeconds :type Float%20%28single-precision%29))
  (bind _owner (Variables|Default|GetOwner))
  (bind _returnvalue (Transformation|GetActorLocation _owner))
  (bind _outhit (Collision|LineTraceByChannel _returnvalue (+ _returnvalue (* (select (Variables|Default|GetOwner%20Was%20Valid%20Pawn) (Math|Vector|GetForwardVector (Pawn|GetControlRotation (Variables|Default|GetOwner%20As%20Pawn) :!class /Script/Engine.Pawn)) (Transformation|GetActorForwardVector (Variables|Default|GetOwner))) (Variables|Default|GetPick%20Up%20Distance))) "TraceTypeQuery1" false 0 "None"))
  (Variables|Default|SetHitting%20Actor (.HitActor (Collision|BreakHitResult _outhit))))

(event EventBeginPlay
  (bind _output_get (Variables|Default|SetOwner (Components|GetOwner)))
  (bind _aspawn (Utilities|Casting|CastToPawn _output_get))
  (bind _output_get_2 (Variables|Default|SetOwner%20As%20Pawn _aspawn))
  (Variables|Default|SetOwner%20Was%20Valid%20Pawn (Utilities|IsValid _output_get_2)))

(fn TryPickUp
  (Class|BPIPickUppable|PickUp(Message) (Variables|Default|GetHitting%20Actor) (Components|GetOwner)))